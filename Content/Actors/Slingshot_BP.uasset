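; Slingshot actor Blueprint that supplies the audio for stretching and launching rocks, with empty event and construction graphs.
; SpawnStretchSound attaches the stretch sound to Holder and returns the spawned component.
; PauseStretchSound pauses the stored stretch component unless already flagged as paused, returning false only when that component is invalid.
; PlayLaunchRockSound calls its parent implementation, then spawns the launch sound on Holder with its own volume multiplier.
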(event `self.ReceiveTick`
  (params (DeltaSeconds :type "Float (single-precision)")))

(fn `pauseStretchSound`
  (returns (ReturnValue :type Boolean))
  (bind _stretchsoundcomp (`self.stretchSoundComp`))
  (`/Engine/EditorBlueprintResources/StandardMacros.IsValid` _stretchsoundcomp
    (:`Is Valid`
      (if (`self.bIsStretchSoundPaused`)
        (return true)
        (else
          (`AudioComponent.SetPaused` _stretchsoundcomp true)
          (return true))))
    (:`Is Not Valid`
      (return false))))

(fn `playLaunchRockSound`
  (`parent.playLaunchRockSound`)
  (`GameplayStatics.SpawnSoundAttached` (`self.rockLaunchSound`) (`self.holder`) "None" (0.0 0.0 0.0) (struct) "KeepRelativeOffset" false (`self.volMult_LaunchSound`) 1.0 0.0 null null)
  (return))

(fn `spawnStretchSound`
  (returns (ReturnValue :type "AudioComponent Object Reference"))
  (bind _returnvalue (`GameplayStatics.SpawnSoundAttached` (`self.stretchSound`) (`self.holder`) "None" (0.0 0.0 0.0) (struct) "KeepRelativeOffset" false (`self.volMult_StretchSound`) 1.0 0.0 null null))
  (return _returnvalue))

(fn `UserConstructionScript`)