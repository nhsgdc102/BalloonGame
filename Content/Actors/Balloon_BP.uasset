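; Balloon target actor that floats upward, scoring when hit by a MovableRock and counting as escaped when it leaves a TriggerBox.
; Both outcomes report to Balloon_GI and call CallDeath with a flag; a rock hit also destroys the rock and detaches the string's start.
; BeginPlay spawns an indicator above it that is removed on Destroyed, and DebugMode disables the rise.
; Construction creates a pop material instance, positions the cable string and only prints a distance-based substep value.
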(event `self.ReceiveBeginPlay`
  (if (`self.bDebugMode`)
    (`ActorComponent.SetActive` (`self.balloonUpwardMovement`) false false))
  (bind _returnvalue (`|SpawnActorFromClass` "/Game/Actors/SpawnIndicator_BP.SpawnIndicator_BP_C" (`KismetMathLibrary.MakeTransform` (+ (`self.K2_GetActorLocation`) (0.0 0.0 109.0))) "AlwaysSpawn" "OverrideRootScale" null null))
  (set `self.SpawnIndicator` _returnvalue))

(event `self.ReceiveTick`
  (params (DeltaSeconds :type "Float (single-precision)")))

(event `self.balloonMesh.OnComponentHit`
  (params (HitComponent :type "PrimitiveComponent Object Reference") (OtherActor :type "Actor Object Reference") (OtherComp :type "PrimitiveComponent Object Reference") (NormalImpulse :type "Vector Structure") (Hit :type "HitResult Structure (by ref)"))
  (if (not (`self.bDead`))
    (`/Game/MacroLibrary_BP.printDebugCollision` (`self.bDebugCollision`) self "Hit" OtherActor
      (:`OutExec`
        (`/Engine/EditorBlueprintResources/StandardMacros.IsValid` OtherActor
          (:`Is Valid`
            (bind _asmovable_rock (cast `MovableRock` OtherActor))
            (set `self.rockVelocity` (`MovementComponent.Velocity` (`MovableRock.rockMovement` _asmovable_rock)))
            (`self.K2_DestroyActor` _asmovable_rock)
            (bind _asballoon_gi (cast `Balloon_GI` (`GameplayStatics.GetGameInstance`)))
            (`Balloon_GI.addToScore` _asballoon_gi (`self.scoreAddition`))
            (set `CableComponent.bAttachStart` false (`self.balloonString`))
            (`self.callDeath` true)))))))

(event `self.balloonMesh.OnComponentEndOverlap`
  (params (OverlappedComponent :type "PrimitiveComponent Object Reference") (OtherActor :type "Actor Object Reference") (OtherComp :type "PrimitiveComponent Object Reference") (OtherBodyIndex :type Integer))
  (if (not (`self.bDead`))
    (`/Game/MacroLibrary_BP.printDebugCollision` (`self.bDebugCollision`) self "EndOverlap" OtherActor
      (:`OutExec`
        (cast `TriggerBox` OtherActor)
        (bind _asballoon_gi (cast `Balloon_GI` (`GameplayStatics.GetGameInstance`)))
        (`Balloon_GI.incrementEscaped` _asballoon_gi)
        (`self.callDeath` false)))))

(event `self.ReceiveDestroyed`
  (bind _spawnindicator (`self.SpawnIndicator`))
  (`/Engine/EditorBlueprintResources/StandardMacros.IsValid` _spawnindicator
    (:`Is Valid`
      (`self.K2_DestroyActor` _spawnindicator))))

(fn `GetCableSubstep`
  (returns (SubstepTime :type "Float (double-precision)"))
  (bind _closecablesubstep (`self.CloseCableSubstep`))
  (return (+ (* (`self.GetHorizontalDistanceTo` (`GameplayStatics.GetPlayerPawn` 0)) (/ (- (`self.FarCableSubstep`) _closecablesubstep) 1000.0)) _closecablesubstep)))

(fn `UserConstructionScript`
  (bind _balloonmesh (`self.balloonMesh`))
  (bind _returnvalue (`PrimitiveComponent.CreateDynamicMaterialInstance` _balloonmesh 0 (`PrimitiveComponent.GetMaterial` _balloonmesh 0) "None"))
  (set `self.DynamicPopInstance` _returnvalue)
  (`KismetSystemLibrary.PrintText` (`KismetTextLibrary.Conv_DoubleToText` (`self.GetCableSubstep`) "HalfToEven"))
  (`SceneComponent.K2_SetWorldLocation` (`self.balloonString`) (`SceneComponent.GetSocketLocation` (`self.balloonMesh`) "CableStart") false false))