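; Slingshot player controller for a balloon-pop game that manages on-screen widgets and screen fade transitions.
; On BeginPlay it optionally creates balloon direction and info display widgets, fades in the BalloonPop HUD and sets Game-and-UI input focused on the info display.
; It forwards zone indices to the direction widget and fades out the HUD for the next level.
; The construction script sets pull sensitivity from the controlled slingshot's minimum displacement, keeping that displacement reachable.
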(event `self.ReceiveBeginPlay`
  (if (`self.bShowBalloonZones`)
    (bind _returnvalue (`|CreateWidget` "/Game/UI/InGame/Zones/BalloonDirection.BalloonDirection_C" self))
    (bind _output_get (set `self.uBalloonZone` _returnvalue))
    (`UserWidget.AddToViewport` _output_get 0))
  (if (`self.bShowInfoDisplay`)
    (bind _returnvalue_2 (`|CreateWidget` "/Game/UI/InGame/InfoDisplay.InfoDisplay_C" self))
    (`UserWidget.AddToViewport` _returnvalue_2 1))
  (bind _asballoon_pop_hud (cast `BalloonPop_HUD` (`self.GetHUD`)))
  (`BalloonPop_HUD.fadeIn` _asballoon_pop_hud)
  (`WidgetBlueprintLibrary.SetInputMode_GameAndUIEx` self _returnvalue_2))

(event `self.DisplayBalloonZone`
  (params (zoneIndex :type Integer))
  (bind _uballoonzone (`self.uBalloonZone`))
  (`/Engine/EditorBlueprintResources/StandardMacros.IsValid` _uballoonzone
    (:`Is Valid`
      (`/Game/UI/InGame/Zones/BalloonDirection.DisplayZone` _uballoonzone zoneIndex))))

(fn `toNextLevel`
  (bind _asballoon_pop_hud (cast `BalloonPop_HUD` (`self.GetHUD`)))
  (`BalloonPop_HUD.fadeOut` _asballoon_pop_hud))

(fn `UserConstructionScript`
  ;[1 1 1] Makes sure inputs allow player to reach minimum displacement
  (bind _asslingshot (cast `Slingshot` (`self.K2_GetPawn`)))
  (set `self.pullSensitivity` (`Slingshot.minimumDisplacement` _asslingshot)) ; 1*pullSensitivity = maximum input
)