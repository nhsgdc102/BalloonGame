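; Iceberg floor actor that rocks back and forth to mimic floating on water.
; Each tick it advances a timer wrapped by Period and passes it to GetRotationRate, a cosine simple-harmonic-motion function scaled by Amplitude.
; The result drives both roll and pitch of the RotatingMovement component's rotation rate, with no yaw.
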(event `self.ReceiveTick`
  (params (DeltaSeconds :type "Float (single-precision)"))
  (bind _output_get (set `self.timePassed` (mod (+ DeltaSeconds (`self.timePassed`)) (`self.period`))))
  (bind _rotrate (`self.getRotationRate` _output_get))
  (set `RotatingMovementComponent.RotationRate` (`KismetMathLibrary.MakeRotator` _rotrate _rotrate) (`self.RotatingMovement`)))

(fn `getRotationRate`
  (params (currentTime :type "Float (double-precision)"))
  (returns (rotRate :type "Float (double-precision)"))
  (return (* (`KismetMathLibrary.Cos` (/ (* (`KismetMathLibrary.MultiplyByPi` currentTime) 2.0) (`self.period`))) (`self.amplitude`))))

(fn `UserConstructionScript`)