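; Game mode Blueprint that handles game over and level transitions, working with a slingshot player controller.
; EndGame deletes the game-status save so the run cannot be resumed, pauses, swaps all widgets for the end screen in UI-only input, and saves play information for the high score.
; StartLevelTransition calls ToNextLevel on the controller, then opens the indexed level from LevelArray after a timer matched to the fade-out.
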(event `self.endGame`
  (bind _returnvalue (`GameplayStatics.GetPlayerController` 0))
  ;[1 1 1] Prevents player from returning to this point in game
  (bind _returnvalue_2 (`GameplayStatics.DoesSaveGameExist` "gameStatusSlot"))
  (if _returnvalue_2
    (`GameplayStatics.DeleteGameInSlot` "gameStatusSlot"))
  (`GameplayStatics.SetGamePaused` true)
  (`WidgetLayoutLibrary.RemoveAllWidgets`) ; Takes out touch interface and info display
  (bind _returnvalue_3 (`|CreateWidget` "/Game/UI/EndScreen/EndGame.EndGame_C" _returnvalue))
  (`UserWidget.AddToViewport` _returnvalue_3 10)
  (`WidgetBlueprintLibrary.SetInputMode_UIOnlyEx` _returnvalue _returnvalue_3)
  ;[1 1 1] Save High Score
  (`self.savePlayInformation`))

(event `self.startLevelTransition`
  (bind _asslingshot_player_bp (cast `/Game/SlingshotPlayer_BP` (`GameplayStatics.GetPlayerController` 0)))
  (`/Game/SlingshotPlayer_BP.toNextLevel` _asslingshot_player_bp)
  (`KismetSystemLibrary.K2_SetTimerDelegate` (delegate `openNextLevel`) 4.0) ; Same Delay as Fade Out Duration
)

(event `self.ReceiveTick`
  (params (DeltaSeconds :type "Float (single-precision)")))

(event `openNextLevel`
  (`GameplayStatics.OpenLevel` (`|GetArrayItem` (`self.levelArray`) (`self.getLevelIndex`))))

(fn `UserConstructionScript`)